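; Flashlight battery inventory item that recharges the player's flashlight when used.
; On use, it adds its battery amount through the player's flashlight component, but only when the current charge is below maximum.
; A successful use flags success and notifies the game state to complete the "UseBattery" objective; a full battery flags the use as failed.
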(event `self.UseItem`
  (bind _bpc_flashlight (`/Game/Blueprints/level1/HG_Character.BPC_FlashLight` (`self.Player Ref`)))
  (if (< (`/Game/Blueprints/blueprintComponents/BPC_FlashLight.CurrentBatteryLevel` _bpc_flashlight) (`/Game/Blueprints/blueprintComponents/BPC_FlashLight.MaxBatteryLevel` _bpc_flashlight))
    (`/Game/Blueprints/blueprintComponents/BPC_FlashLight.AddBatteryLife` _bpc_flashlight (`self.BatteryAmount`))
    (set `self.UseItemSuccess` true)
    (message `/Game/Blueprints/Interface/BPI_ObjectiveCall.CompleteObjectiveCall` (`GameplayStatics.GetGameState`) "UseBattery" false)
    (else
      (set `self.UseItemSuccess` false))))

(fn `UserConstructionScript`
  (`parent.UserConstructionScript`))