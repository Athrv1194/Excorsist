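; BP_InventoryBackPack is a world pickup that adds slots to the player's inventory when collected, then destroys itself.
; Overlapping its sphere shows a floating prompt widget and starts a Tick check that line-traces to the player's camera.
; With clear line of sight, the widget faces the camera, and its prompt and the actor's input are toggled by pickup distance, so the Action key only works up close.
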(event `self.Sphere.OnComponentBeginOverlap`
  (params (OverlappedComponent :type "PrimitiveComponent Object Reference") (OtherActor :type "Actor Object Reference") (OtherComp :type "PrimitiveComponent Object Reference") (OtherBodyIndex :type Integer) (bFromSweep :type Boolean) (SweepResult :type "HitResult Structure (by ref)"))
  (bind _ashg_character (cast `/Game/Blueprints/level1/HG_Character` OtherActor))
  (set `self.PlayerRef` _ashg_character)
  (`SceneComponent.SetVisibility` (`self.PickupWidget`) true false)
  (set `self.UpdateActor` true))

(event `self.Sphere.OnComponentEndOverlap`
  (params (OverlappedComponent :type "PrimitiveComponent Object Reference") (OtherActor :type "Actor Object Reference") (OtherComp :type "PrimitiveComponent Object Reference") (OtherBodyIndex :type Integer))
  (cast `/Game/Blueprints/level1/HG_Character` OtherActor)
  (`SceneComponent.SetVisibility` (`self.PickupWidget`) false false)
  (set `self.UpdateActor` false)
  (`self.DisableInput` (`GameplayStatics.GetPlayerController` 0)))

(event `self.ReceiveTick`
  (params (DeltaSeconds :type "Float (single-precision)"))
  (bind _returnvalue (`GameplayStatics.GetPlayerController` 0))
  (bind _pickupwidget (`self.PickupWidget`))
  (bind (_returnvalue_x _returnvalue_y _returnvalue_z) (`KismetMathLibrary.BreakVector` (`SceneComponent.K2_GetComponentLocation` (`self.BackPackMesh`))))
  (`SceneComponent.K2_SetWorldLocation` (`self.PickupWidget`) (`KismetMathLibrary.MakeVector` _returnvalue_x _returnvalue_y (+ _returnvalue_z (`self.WidgetDistanceAboveMesh`))) false false)
  (if (`self.UpdateActor`)
    (bind (_outhit _returnvalue_2) (`KismetSystemLibrary.LineTraceSingle` :`Start` (`self.K2_GetActorLocation`) :`End` (`SceneComponent.K2_GetComponentLocation` (`/Game/Blueprints/level1/HG_Character.Camera` (`self.PlayerRef`))) :`TraceChannel` "TraceTypeQuery1" :`DrawDebugType` "ForOneFrame"))
    (if (not _returnvalue_2)
      (`SceneComponent.SetVisibility` _pickupwidget true false)
      (`SceneComponent.K2_SetWorldRotation` (`self.PickupWidget`) (`KismetMathLibrary.FindLookAtRotation` (`SceneComponent.K2_GetComponentLocation` (`self.PickupWidget`)) (`SceneComponent.K2_GetComponentLocation` (`/Game/Blueprints/level1/HG_Character.Camera` (`self.PlayerRef`)))) false false)
      (bind (_bblockinghit _binitialoverlap _time _distance _location _impactpoint _normal _impactnormal _physmat _hitactor _hitcomponent _hitbonename _bonename _hititem _elementindex _faceindex _tracestart _traceend) (`GameplayStatics.BreakHitResult` _outhit))
      (bind _returnvalue_3 (<= (`KismetMathLibrary.VSize` (- _tracestart _traceend)) (`self.PickUpDistance`)))
      (`/Game/UMG/Inventory/W_Inventory_PickUpPrompt.TogglePrompt` (cast `/Game/UMG/Inventory/W_Inventory_PickUpPrompt` (`WidgetComponent.GetUserWidgetObject` (`self.PickupWidget`)) :!pure true) _returnvalue_3)
      (if _returnvalue_3
        (`self.EnableInput` _returnvalue)
        (else
          (`self.DisableInput` _returnvalue)))
      (else
        (`SceneComponent.SetVisibility` _pickupwidget false false)
        (`self.DisableInput` (`GameplayStatics.GetPlayerController` 0))))))

(event `InputAction|Action`
  (params (Key :type "Key Structure"))
  (:`Pressed`
    (`/Game/Blueprints/blueprintComponents/BPC_Inventory.AddMoreSlots` (`/Game/Blueprints/level1/HG_Character.BPC_Inventory` (`self.PlayerRef`)) (`self.AmountOfSlots`))
    (`self.K2_DestroyActor`)))

(fn `UserConstructionScript`)