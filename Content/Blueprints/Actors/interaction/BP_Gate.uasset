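; BP_Gate is an interactable gate that the player can toggle open or closed and that opens automatically for AI_Classic actors.
; Interact plays or reverses a timeline sliding the mesh along local X, its direction chosen by a facing dot product against the player.
; The box overlap instead drives a second timeline that swings the mesh in yaw away from the AI, blocking interaction until that timeline finishes closing.
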(event `/Game/Blueprints/Interface/BPI_Interaction.Interact`
  (if (`self.canInteract`)
    (if (`self.isDoorClosed`)
      (set `self.isDoorClosed` false)
      (set `self.DotProduct` (`KismetMathLibrary.Dot_VectorVector` (`KismetMathLibrary.Normal` (- (`self.K2_GetActorLocation` self) (`self.K2_GetActorLocation` (`self.PlayerRef`)))) (`self.GetActorForwardVector` self)))
      (bind (_direction _alpha) (`Timeline|OpenDoorTL` :!via `PlayFromStart` :!label _label)
        (:`Update`
          (`SceneComponent.K2_SetRelativeLocation` (`self.StaticMesh1`) (`KismetMathLibrary.MakeVector` (`KismetMathLibrary.Lerp` 0.0 (select `bool` (>= (`self.DotProduct`) 0.0) :`false` -90.0 :`true` 90.0) _alpha)) false false)))
      (else
        (set `self.isDoorClosed` true)
        (goto _label :!via `ReverseFromEnd`)))))

(event `self.Box.OnComponentBeginOverlap`
  (params (OverlappedComponent :type "PrimitiveComponent Object Reference") (OtherActor :type "Actor Object Reference") (OtherComp :type "PrimitiveComponent Object Reference") (OtherBodyIndex :type Integer) (bFromSweep :type Boolean) (SweepResult :type "HitResult Structure (by ref)"))
  (bind _asai_classic (cast `/Game/AI/AIClassic/AI_Classic` OtherActor))
  (set `self.canInteract` false)
  (if (`self.isDoorClosed`)
    (set `self.isDoorClosed` false)
    (set `self.DotProduct` (`KismetMathLibrary.Dot_VectorVector` (`KismetMathLibrary.Normal` (- (`self.K2_GetActorLocation` self) (`self.K2_GetActorLocation` _asai_classic))) (`self.GetActorForwardVector` self)))
    (bind (_direction _alpha) (`Timeline|OpenDoorAI` :!via `PlayFromStart` :!label _label_2)
      (:`Update`
        (`SceneComponent.K2_SetRelativeRotation` (`self.StaticMesh1`) (`KismetMathLibrary.MakeRotator` 0.0 0.0 (`KismetMathLibrary.Lerp` 0.0 (select `bool` (>= (`self.DotProduct`) 0.0) :`false` -90.0 :`true` 90.0) _alpha)) false false))
      (:`Finished`
        (switch `ETimelineDirection` _direction
          (:`Backward`
            (set `self.canInteract` true)))))))

(event `self.Box.OnComponentEndOverlap`
  (params (OverlappedComponent :type "PrimitiveComponent Object Reference") (OtherActor :type "Actor Object Reference") (OtherComp :type "PrimitiveComponent Object Reference") (OtherBodyIndex :type Integer))
  (cast `/Game/AI/AIClassic/AI_Classic` OtherActor)
  (if (not (`self.isDoorClosed`))
    (set `self.isDoorClosed` true)
    (goto _label_2 :!via `ReverseFromEnd`)))

(fn `UserConstructionScript`
  (`parent.UserConstructionScript`))