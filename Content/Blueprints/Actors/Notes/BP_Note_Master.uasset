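; BP_Note_Master is a base note actor that shows front and back text, set at construction, and can be opened for examination.
; Overlapping HG_Character enables a per-tick line trace to the player camera.
; With clear line of sight, a prompt faces the camera, and input is enabled within pickup distance.
; The Action input opens a W_NoteExamination widget, passing it this note and the level's BP_NoteExamination.
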(event `self.ReceiveBeginPlay`
  (bind _outactors (`GameplayStatics.GetAllActorsOfClass` "/Game/Blueprints/Actors/Notes/BP_NoteExamination.BP_NoteExamination_C"))
  (set `self.BPNoteExaminationRef` (`|GetArrayItem` _outactors)))

(event `self.OverlapSphere.OnComponentBeginOverlap`
  (params (OverlappedComponent :type "PrimitiveComponent Object Reference") (OtherActor :type "Actor Object Reference") (OtherComp :type "PrimitiveComponent Object Reference") (OtherBodyIndex :type Integer) (bFromSweep :type Boolean) (SweepResult :type "HitResult Structure (by ref)"))
  (bind _ashg_character (cast `/Game/Blueprints/level1/HG_Character` OtherActor))
  (set `self.PlayerRef` _ashg_character)
  (`SceneComponent.SetVisibility` (`self.PromptWidget`) true false)
  (set `self.UpdateActor` true))

(event `self.OverlapSphere.OnComponentEndOverlap`
  (params (OverlappedComponent :type "PrimitiveComponent Object Reference") (OtherActor :type "Actor Object Reference") (OtherComp :type "PrimitiveComponent Object Reference") (OtherBodyIndex :type Integer))
  (cast `/Game/Blueprints/level1/HG_Character` OtherActor)
  (`SceneComponent.SetVisibility` (`self.PromptWidget`) false false)
  (set `self.UpdateActor` false)
  (`self.DisableInput` (`GameplayStatics.GetPlayerController` 0)))

(event `self.ReceiveTick`
  (params (DeltaSeconds :type "Float (single-precision)"))
  (bind _returnvalue (`GameplayStatics.GetPlayerController` 0))
  (bind _promptwidget (`self.PromptWidget`))
  (bind (_returnvalue_x _returnvalue_y _returnvalue_z) (`KismetMathLibrary.BreakVector` (`SceneComponent.K2_GetComponentLocation` (`self.Paper`))))
  (`SceneComponent.K2_SetWorldLocation` (`self.PromptWidget`) (`KismetMathLibrary.MakeVector` _returnvalue_x _returnvalue_y (+ _returnvalue_z (`self.WidgetDistanceAboveMesh`))) false false)
  (if (`self.UpdateActor`)
    (bind (_outhit _returnvalue_2) (`KismetSystemLibrary.LineTraceSingle` :`Start` (`self.K2_GetActorLocation`) :`End` (`SceneComponent.K2_GetComponentLocation` (`/Game/Blueprints/level1/HG_Character.Camera` (`self.PlayerRef`))) :`TraceChannel` "TraceTypeQuery1" :`DrawDebugType` "ForOneFrame"))
    (if (not _returnvalue_2)
      (`SceneComponent.SetVisibility` _promptwidget true false)
      (`SceneComponent.K2_SetWorldRotation` (`self.PromptWidget`) (`KismetMathLibrary.FindLookAtRotation` (`SceneComponent.K2_GetComponentLocation` (`self.PromptWidget`)) (`SceneComponent.K2_GetComponentLocation` (`/Game/Blueprints/level1/HG_Character.Camera` (`self.PlayerRef`)))) false false)
      (bind (_bblockinghit _binitialoverlap _time _distance _location _impactpoint _normal _impactnormal _physmat _hitactor _hitcomponent _hitbonename _bonename _hititem _elementindex _faceindex _tracestart _traceend) (`GameplayStatics.BreakHitResult` _outhit))
      (bind _returnvalue_3 (<= (`KismetMathLibrary.VSize` (- _tracestart _traceend)) (`self.PickUpDistance`)))
      (`/Game/UMG/Inventory/W_Inventory_PickUpPrompt.TogglePrompt` (cast `/Game/UMG/Inventory/W_Inventory_PickUpPrompt` (`WidgetComponent.GetUserWidgetObject` (`self.PromptWidget`)) :!pure true) _returnvalue_3)
      (if _returnvalue_3
        (`self.EnableInput` _returnvalue)
        (else
          (`self.DisableInput` _returnvalue)))
      (else
        (`SceneComponent.SetVisibility` _promptwidget false false)
        (`self.DisableInput` (`GameplayStatics.GetPlayerController` 0))))))

(event `InputAction|Action`
  (params (Key :type "Key Structure"))
  (:`Pressed`
    (bind _returnvalue (`|CreateWidget` "/Game/UMG/W_NoteExamination.W_NoteExamination_C" null (`self.BPNoteExaminationRef`)))
    (`/Game/UMG/W_NoteExamination.UpdateWidget` _returnvalue self)
    (`UserWidget.AddToViewport` _returnvalue 0)))

(fn `UserConstructionScript`
  (`TextRenderComponent.K2_SetText` (`self.NoteRender`) (`self.NoteText`))
  (`TextRenderComponent.K2_SetText` (`self.NoteRenderBack`) (`self.BackNoteText`)))