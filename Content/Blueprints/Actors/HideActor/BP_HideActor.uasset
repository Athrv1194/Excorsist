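; Hiding spot actor that the player interacts with to slip into or out of cover from the enemy.
; Interact starts a frame-interval looping timer that slides the player at constant speed to the hiding or exit point, chosen by IsHiding.
; Entering alerts the AIC_Classic controller and disables collision, movement and inventory.
; On arrival it fires a dispatcher and flips IsHiding, with exits also notifying the AI and restoring control.
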(event `self.ReceiveBeginPlay`
  (bind _ashg_character (cast `/Game/Blueprints/level1/HG_Character` (`GameplayStatics.GetPlayerCharacter` 0)))
  (set `self.PlayerRef` _ashg_character)
  (bind _ashg_player_controller (cast `/Game/Blueprints/HG_PlayerController` (`GameplayStatics.GetPlayerController` 0)))
  (set `self.ControllerRef` _ashg_player_controller))

(event `/Game/Blueprints/Interface/BPI_Interaction.Interact`
  (bind _playerref (`self.PlayerRef`))
  (if (`/Game/Blueprints/level1/HG_Character.isHiding` (`self.PlayerRef`))
    (bind _returnvalue (`KismetSystemLibrary.K2_SetTimerDelegate` (delegate `MoveCharacter`) (`GameplayStatics.GetWorldDeltaSeconds`) true))
    (else
      (bind _asaic_classic (castclass `/Game/AI/AIClassic/AIC_Classic` "/Game/AI/AIClassic/AIC_Classic.AIC_Classic_C"))
      (bind _returnvalue_2 (`GameplayStatics.GetActorOfClass` _asaic_classic))
      (message `/Game/Blueprints/Interface/BPI_PlayerHiding.DidEnemySee` _returnvalue_2 self)
      (`self.SetActorEnableCollision` _playerref false)
      (`CharacterMovementComponent.DisableMovement` (`Character.CharacterMovement` _playerref))
      (set `/Game/Blueprints/HG_PlayerController.canOpenInventory` false (`self.ControllerRef`))
      (bind _returnvalue_3 (`KismetSystemLibrary.K2_SetTimerDelegate` (delegate `MoveCharacter`) (`GameplayStatics.GetWorldDeltaSeconds`) true)))))

(event `MoveCharacter`
  (bind _playerref (`self.PlayerRef`))
  (`self.K2_SetActorTransform` _playerref (`KismetMathLibrary.MakeTransform` (`KismetMathLibrary.VInterpTo_Constant` (`self.K2_GetActorLocation` _playerref) (`SceneComponent.K2_GetComponentLocation` (select `bool` (`/Game/Blueprints/level1/HG_Character.isHiding` (`self.PlayerRef`)) :`false` (`self.HidingPosition`) :`true` (`self.ExitPosition`) :!type "SceneComponent Object Reference")) (`GameplayStatics.GetWorldDeltaSeconds`) 1000.0)) false false)
  (if (`KismetMathLibrary.EqualExactly_VectorVector` (`self.K2_GetActorLocation` (`self.PlayerRef`)) (`SceneComponent.K2_GetComponentLocation` (select `bool` (`/Game/Blueprints/level1/HG_Character.isHiding` (`self.PlayerRef`)) :`false` (`self.HidingPosition`) :`true` (`self.ExitPosition`) :!type "SceneComponent Object Reference")))
    (`KismetSystemLibrary.K2_ClearAndInvalidateTimerHandle` (stale `/Game/Blueprints/Interface/BPI_Interaction.Interact` _returnvalue_3))
    (`KismetSystemLibrary.K2_ClearAndInvalidateTimerHandle` (stale `/Game/Blueprints/Interface/BPI_Interaction.Interact` _returnvalue))
    (`self.FinishedMoving`)))

(event `FinishedMoving`
  (bind _playerref (`self.PlayerRef`))
  (bind _playerref_2 (`self.PlayerRef`))
  (`self.FinishedMovingED`)
  (if (`/Game/Blueprints/level1/HG_Character.isHiding` _playerref)
    (set `/Game/Blueprints/level1/HG_Character.isHiding` false _playerref)
    (bind _asaic_classic (castclass `/Game/AI/AIClassic/AIC_Classic` "/Game/AI/AIClassic/AIC_Classic.AIC_Classic_C"))
    (bind _returnvalue (`GameplayStatics.GetActorOfClass` _asaic_classic))
    (message `/Game/Blueprints/Interface/BPI_PlayerHiding.LeftHidingSpot` _returnvalue)
    (`self.SetActorEnableCollision` _playerref_2 true)
    (`CharacterMovementComponent.SetMovementMode` (`Character.CharacterMovement` _playerref_2) "MOVE_Walking" 0)
    (set `/Game/Blueprints/HG_PlayerController.canOpenInventory` true (`self.ControllerRef`))
    (else
      (set `/Game/Blueprints/level1/HG_Character.isHiding` true _playerref))))

(event `EnemyFound`)

(fn `UserConstructionScript`)