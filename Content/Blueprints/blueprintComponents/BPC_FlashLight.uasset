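; Flashlight component that toggles the player's FlashLight light and manages its battery life.
; Initialize caches the light; toggling it on requires remaining charge and starts a looping timer that drains the battery, switching the light off at minimum.
; Battery changes, including recharges through AddBatteryLife, update the IES brightness scale via a clamped range map, so dimming only occurs at low charge.
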(fn `AddBatteryLife`
  (params (Amount :type "Float (double-precision)"))
  (set `self.CurrentBatteryLevel` (`KismetMathLibrary.FClamp` (+ Amount (`self.CurrentBatteryLevel`)) (`self.MinBatteryLevel`) (`self.MaxBatteryLevel`)))
  (`self.SetIntensity`))

(fn `DepleteBatteryLife`
  (bind _output_get (set `self.CurrentBatteryLevel` (`KismetMathLibrary.FClamp` (- (`self.CurrentBatteryLevel`) (`self.DepletionAmount`)) (`self.MinBatteryLevel`) (`self.MaxBatteryLevel`))))
  (`self.SetIntensity`)
  (if (<= _output_get (`self.MinBatteryLevel`))
    (`SceneComponent.SetVisibility` (`self.Light`) false false)
    (`KismetSystemLibrary.K2_ClearTimer` null "DepleteBatteryLife")))

(fn `Initialize`
  (params (Player :type "/Game/Blueprints/level1/HG_Character Object Reference"))
  (bind _output_get (set `self.Player Ref` Player))
  (set `self.Light` (`/Game/Blueprints/level1/HG_Character.FlashLight` _output_get)))

(fn `SetIntensity`
  (`LightComponent.SetIESBrightnessScale` (`self.Light`) (`KismetMathLibrary.MapRangeClamped` (`self.CurrentBatteryLevel`) (`self.MinBatteryLevel`) 20.0 0.0 1.0)))

(fn `ToggleFlashLight`
  (bind _light (`self.Light`))
  (if (`SceneComponent.bVisible` _light)
    (`SceneComponent.SetVisibility` _light false false)
    (`KismetSystemLibrary.K2_ClearTimer` null "DepleteBatteryLife")
    (elif (> (`self.CurrentBatteryLevel`) (`self.MinBatteryLevel`))
      (`self.SetIntensity`)
      (`SceneComponent.SetVisibility` _light true false)
      (`KismetSystemLibrary.K2_SetTimer` null "DepleteBatteryLife" (`self.DepletionSpeed`) true))))