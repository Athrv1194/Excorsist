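; Inventory component that stores items in a resizable slot array sized from HG_PlayerController and refreshes the inventory grid widget as slots change.
; AddItem fills partial stacks, then empty slots, recursing for overflow.
; UseItem calls an existing or newly spawned item actor and consumes one on success.
; DropItem spawns a physics pickup at a camera trace point, and an examination widget created at startup displays selected items.
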(event `self.ReceiveBeginPlay`
  (`self.Initialize`))

(event `Initialize`
  (bind _ashg_player_controller (cast `/Game/Blueprints/HG_PlayerController` (`GameplayStatics.GetPlayerController` 0) :!pure true))
  (`KismetArrayLibrary.Array_Resize` (`self.InventorySlots`) (`/Game/Blueprints/HG_PlayerController.InventorySlots` _ashg_player_controller))
  (set `self.W Inventory Menu Ref` (`/Game/Blueprints/HG_PlayerController.W_InventoryMenuRef` _ashg_player_controller))
  (bind _ashg_character (cast `/Game/Blueprints/level1/HG_Character` (`GameplayStatics.GetPlayerCharacter` 0)))
  (set `self.PlayerRef` _ashg_character)
  (bind _returnvalue (`|CreateWidget` "/Game/UMG/Inventory/W_Examination.W_Examination_C" null null))
  (set `self.WExaminationRef` _returnvalue)
  (set `/Game/Blueprints/HG_PlayerController.W_ExaminationRef` (`self.WExaminationRef`) _ashg_player_controller)
  (bind _outactors (`GameplayStatics.GetAllActorsOfClass` "/Game/Blueprints/Actors/Inventory/BP_Examination.BP_Examination_C"))
  (set `self.BP_ExaminationRef` (`|GetArrayItem` _outactors))
  (set `/Game/UMG/Inventory/W_Examination.BPC_InventoryRef` self (`self.WExaminationRef`)))

(event `CreateExaminationWidget`
  (params (Index :type Integer))
  (bind _w_inventory_menu_ref (`self.W Inventory Menu Ref`))
  (`/Game/UMG/Inventory/W_Examination.UpdateWidget` (`self.WExaminationRef`) Index)
  (`Widget.SetVisibility` _w_inventory_menu_ref "Collapsed")
  (`/Engine/EditorBlueprintResources/StandardMacros.IsValid` (`/Game/UMG/Inventory/W_InventoryMenu.W_Inventory_DropDown_1` _w_inventory_menu_ref)
    (:`Is Valid`
      (`/Game/UMG/Inventory/W_InventoryMenu.CloseDropDownMenu` _w_inventory_menu_ref))
    (:`Is Not Valid`
      _))
  (`UserWidget.AddToViewport` (`self.WExaminationRef`) 2)
  (set `/Game/Blueprints/HG_PlayerController.isInventoryOpen` false (cast `/Game/Blueprints/HG_PlayerController` (`GameplayStatics.GetPlayerController` 0) :!pure true)))

(fn `AddItem`
  (params (Item :type "/Game/Blueprints/Actors/Inventory/BP_InventoryItem_master Class Reference") (Amount :type Integer))
  (returns (`Success?` :type Boolean) (Remainder :type Integer))
  (locals (LocalItem :type "/Game/Blueprints/Actors/Inventory/BP_InventoryItem_master Class Reference") (LocalAmount :type Integer) (LocalMaxStackAmount :type Integer) (LocalIndex :type Integer :default 0))
  (bind (_success_ _index) (`self.CheckForEmptySlot`))
  (bind (_success__2 _index_2) (`self.CheckForEmptySlot`))
  (bind _returnvalue (- (`local.LocalAmount`) 1))
  (bind (_itemname _icon _maxstalkamount) (break `/Game/Blueprints/Structs/S_ItemData` (defaults `Object` (`local.LocalItem`))))
  (bind _returnvalue_2 (+ (`.Amount` (`self.GetItemDataAtIndex` (`local.LocalIndex`))) (`local.LocalAmount`)))
  (set `local.LocalItem` Item)
  (set `local.LocalAmount` Amount)
  (set `local.LocalMaxStackAmount` _maxstalkamount)
  (if (> _maxstalkamount 1)
    (bind (_success__3 _index_3) (`self.CheckForFreeSlot` (`local.LocalItem`)))
    (if _success__3
      (set `local.LocalIndex` _index_3)
      (if (> _returnvalue_2 (`local.LocalMaxStackAmount`))
        (set `local.LocalAmount` (- _returnvalue_2 (`local.LocalMaxStackAmount`)))
        (`KismetArrayLibrary.Array_Set` (`self.InventorySlots`) (`local.LocalIndex`) (make `/Game/Blueprints/Structs/S_InventoryItem` (`local.LocalItem`) (`local.LocalMaxStackAmount`)))
        (`self.UpdateInventorySlot` (`local.LocalIndex`))
        (`self.AddItem` (`local.LocalItem`) (`local.LocalAmount`))
        (else
          (`KismetArrayLibrary.Array_Set` (`self.InventorySlots`) (`local.LocalIndex`) (make `/Game/Blueprints/Structs/S_InventoryItem` (`local.LocalItem`) _returnvalue_2))
          (`self.UpdateInventorySlot` (`local.LocalIndex`))
          (return true 0)))
      (elif _success_
        (set `local.LocalIndex` _index)
        (if (> (`local.LocalAmount`) (`local.LocalMaxStackAmount`))
          (`KismetArrayLibrary.Array_Set` (`self.InventorySlots`) (`local.LocalIndex`) (make `/Game/Blueprints/Structs/S_InventoryItem` (`local.LocalItem`) (`local.LocalAmount`)))
          (`self.UpdateInventorySlot` (`local.LocalIndex`))
          (bind (_success__4 _remainder) (`self.AddItem` (`local.LocalItem`) (- (`local.LocalAmount`) (`local.LocalMaxStackAmount`))))
          (return true _remainder)
          (else
            (`KismetArrayLibrary.Array_Set` (`self.InventorySlots`) (`local.LocalIndex`) (make `/Game/Blueprints/Structs/S_InventoryItem` (`local.LocalItem`) (`local.LocalAmount`)))
            (`self.UpdateInventorySlot` (`local.LocalIndex`))
            (return true 0)))
        (else
          (return false (`local.LocalAmount`)))))
    (elif _success__2
      (set `local.LocalIndex` _index_2)
      (`KismetArrayLibrary.Array_Set` (`self.InventorySlots`) (`local.LocalIndex`) (make `/Game/Blueprints/Structs/S_InventoryItem` (`local.LocalItem`) 1))
      (`self.UpdateInventorySlot` (`local.LocalIndex`))
      (if (> _returnvalue 0)
        (bind (_success__5 _remainder_2) (`self.AddItem` (`local.LocalItem`) _returnvalue))
        (return true _remainder_2)
        (else
          (return true 0)))
      (else
        (`KismetSystemLibrary.PrintString` "No Free Slots Available")
        (return false (`local.LocalAmount`))))))

(fn `AddMoreSlots`
  (params (Amount :type Integer))
  (bind _w_inventory_menu_ref (`self.W Inventory Menu Ref`))
  (bind _ashg_player_controller (cast `/Game/Blueprints/HG_PlayerController` (`GameplayStatics.GetPlayerController` 0) :!pure true))
  (bind _w_inventorygrid (`/Game/UMG/Inventory/W_InventoryMenu.W_InventoryGrid` _w_inventory_menu_ref))
  (bind _output_get (set `/Game/Blueprints/HG_PlayerController.InventorySlots` (+ (`/Game/Blueprints/HG_PlayerController.InventorySlots` _ashg_player_controller) Amount) _ashg_player_controller))
  (`KismetArrayLibrary.Array_Resize` (`self.InventorySlots`) _output_get)
  (`/Game/UMG/Inventory/W_InventoryGrid.AddMoreSlots` _w_inventorygrid Amount)
  (for _array_element (`/Game/UMG/Inventory/W_InventoryGrid.SlotsArray` _w_inventorygrid)
    (`/Game/UMG/Inventory/W_InventorySlots.Intialize` _array_element _w_inventory_menu_ref)))

(fn `CheckForEmptySlot`
  (returns (`Success?` :type Boolean) (Index :type Integer))
  (locals (LocalSuccess :type Boolean) (localIndex :type Integer))
  (for (_array_element _array_index) (`self.InventorySlots`)
    (if (`KismetSystemLibrary.IsValidClass` (`.Item_6_454EB0944BB57657F9AB0A9DF28969C2` (break `/Game/Blueprints/Structs/S_InventoryItem` _array_element)))
      (set `local.LocalSuccess` false)
      (else
        (set `local.LocalSuccess` true)
        (set `local.localIndex` _array_index)
        (break))))
  (return (`local.LocalSuccess`) (`local.localIndex`)))

(fn `CheckForFreeSlot`
  (params (Item :type "/Game/Blueprints/Actors/Inventory/BP_InventoryItem_master Class Reference"))
  (returns (`Success?` :type Boolean) (Index :type Integer))
  (locals (LocalIndex :type Integer) (LocalSuccess :type Boolean))
  (for (_array_element _array_index) (`self.InventorySlots`)
    (bind (_item _amount) (break `/Game/Blueprints/Structs/S_InventoryItem` _array_element))
    (if (and (== _item Item) (< _amount (`.MaxStalkAmount_8_9C92CB9F4C9EBBB767560681437FD5DE` (break `/Game/Blueprints/Structs/S_ItemData` (defaults `Object` Item)))))
      (set `local.LocalSuccess` true)
      (set `local.LocalIndex` _array_index)
      (break)
      (else
        (set `local.LocalSuccess` false))))
  (return (`local.LocalSuccess`) (`local.LocalIndex`)))

(fn `DropItem`
  (params (Index :type Integer))
  (locals (LocalIndex :type Integer) (LocalAmount :type Integer :default 0) (LocalClass :type "/Game/Blueprints/Actors/Inventory/BP_InventoryItem_master Class Reference") (Localfloat :type "Float (double-precision)" :default 200.0) (NewLocalVar :type "/Game/Blueprints/Actors/Inventory/PickupActors/BP_PickupActor_Master Object Reference"))
  (bind _camera (`/Game/Blueprints/level1/HG_Character.Camera` (`self.PlayerRef`)))
  (bind _returnvalue (`SceneComponent.K2_GetComponentLocation` _camera))
  (bind _output_get (set `local.LocalIndex` Index))
  (bind (_item _amount) (`self.GetItemDataAtIndex` _output_get))
  (set `local.LocalAmount` _amount)
  (set `local.LocalClass` _item)
  (if (> (`local.LocalAmount`) 0)
    (for _ (range (`local.LocalAmount`))
      (`self.RemoveItem` (`local.LocalIndex`)))
    (`/Game/UMG/Inventory/W_InventoryMenu.CloseDropDownMenu` (`self.W Inventory Menu Ref`))
    (bind (_outhit _returnvalue_2) (`KismetSystemLibrary.LineTraceSingle` _returnvalue (+ _returnvalue (* (`SceneComponent.GetForwardVector` _camera) (`local.Localfloat`))) "TraceTypeQuery1"))
    (bind (_bblockinghit _binitialoverlap _time _distance _location _impactpoint _normal _impactnormal _physmat _hitactor _hitcomponent _hitbonename _bonename _hititem _elementindex _faceindex _tracestart _traceend) (`GameplayStatics.BreakHitResult` _outhit))
    (bind _returnvalue_3 (`|SpawnActorFromClass` (`.PickupActor_15_14005EF14554CE206A69B5A4C717C2FC` (break `/Game/Blueprints/Structs/S_ItemData` (defaults `Object` (`local.LocalClass`)))) (`KismetMathLibrary.MakeTransform` (select `bool` _returnvalue_2 :`false` _traceend :`true` _location)) "Undefined" "OverrideRootScale" null null))
    (set `/Game/Blueprints/Actors/Inventory/PickupActors/BP_PickupActor_Master.Amount` (`local.LocalAmount`) _returnvalue_3)
    (`PrimitiveComponent.SetSimulatePhysics` (`/Game/Blueprints/Actors/Inventory/PickupActors/BP_PickupActor_Master.StaticMesh` _returnvalue_3) true)))

(fn `GetItemDataAtIndex`
  (params (Index :type Integer))
  (returns (Item :type "/Game/Blueprints/Actors/Inventory/BP_InventoryItem_master Class Reference") (Amount :type Integer))
  (bind (_item _amount) (break `/Game/Blueprints/Structs/S_InventoryItem` (`|GetArrayItem` (`self.InventorySlots`) Index)))
  (return _item _amount))

(fn `RemoveItem`
  (params (Index :type Integer))
  (bind (_item _amount) (`self.GetItemDataAtIndex` Index))
  (if (> _amount 1)
    (`KismetArrayLibrary.Array_Set` (`self.InventorySlots`) Index (make `/Game/Blueprints/Structs/S_InventoryItem` _item (- _amount 1)))
    (else
      (`KismetArrayLibrary.Array_Set` (`self.InventorySlots`) Index (make `/Game/Blueprints/Structs/S_InventoryItem` null))))
  (`self.UpdateInventorySlot` Index))

(fn `UpdateInventorySlot`
  (params (Index :type Integer))
  (`/Game/UMG/Inventory/W_InventorySlots.UpdateSlot` (`|GetArrayItem` (`/Game/UMG/Inventory/W_InventoryGrid.SlotsArray` (`/Game/UMG/Inventory/W_InventoryMenu.W_InventoryGrid` (`/Game/Blueprints/HG_PlayerController.W_InventoryMenuRef` (cast `/Game/Blueprints/HG_PlayerController` (`GameplayStatics.GetPlayerController` 0) :!pure true)))) Index)))

(fn `Use Item`
  (params (Index :type Integer))
  (locals (LocalIndex :type Integer))
  (bind _output_get (set `local.LocalIndex` Index))
  (bind (_item _amount) (`self.GetItemDataAtIndex` _output_get))
  (if (> _amount 0)
    (bind _returnvalue (`GameplayStatics.GetActorOfClass` _item))
    (`/Engine/EditorBlueprintResources/StandardMacros.IsValid` _returnvalue
      (:`Is Valid`
        (`/Game/Blueprints/Actors/Inventory/BP_InventoryItem_master.UseItem` _returnvalue)
        (if (`/Game/Blueprints/Actors/Inventory/BP_InventoryItem_master.UseItemSuccess` _returnvalue)
          (`self.RemoveItem` (`local.LocalIndex`) :!label _label)
          (`/Game/UMG/Inventory/W_InventoryMenu.CloseDropDownMenu` (`self.W Inventory Menu Ref`))
          (else
            (`KismetSystemLibrary.PrintString` "Use Item Not Successful" :!label _label_2))))
      (:`Is Not Valid`
        (bind _returnvalue_2 (`|SpawnActorFromClass` _item (`KismetMathLibrary.MakeTransform` (0.0 0.0 0.0)) "Undefined" "OverrideRootScale" null null))
        (`/Game/Blueprints/Actors/Inventory/BP_InventoryItem_master.UseItem` _returnvalue_2)
        (if (`/Game/Blueprints/Actors/Inventory/BP_InventoryItem_master.UseItemSuccess` _returnvalue_2)
          (goto _label)
          (else
            (goto _label_2)))))))